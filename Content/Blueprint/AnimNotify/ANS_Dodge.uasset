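; ANS_Dodge is an animation notify state that displaces the owning actor during a dodge animation.
; Each notify tick fetches the owner's pre-velocity through GetPreVelocityMessage, scales it by a fixed factor and adds it as a world offset.
; The offset is neither swept for collision nor scaled by frame delta time.
; The IsBackward flag selects between two branches that currently perform identical movement.
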(fn `Received_NotifyTick`
  (params (MeshComp :type "SkeletalMeshComponent Object Reference") (Animation :type "AnimSequenceBase Object Reference") (FrameDeltaTime :type "Float (single-precision)") (EventReference :type "AnimNotifyEventReference Structure (by ref)"))
  (returns (ReturnValue :type Boolean))
  (bind _returnvalue (`ActorComponent.GetOwner` MeshComp))
  (bind _returnvalue_2 (`ActorComponent.GetOwner` MeshComp))
  (if (`self.IsBackward`)
    (bind _returnvalue_3 (message `CharacterInterface.GetPreVelocity` _returnvalue_2))
    (`Actor.K2_AddActorWorldOffset` _returnvalue_2 (* _returnvalue_3 2.5) false false)
    (return false)
    (else
      (bind _returnvalue_4 (message `CharacterInterface.GetPreVelocity` _returnvalue))
      (`Actor.K2_AddActorWorldOffset` _returnvalue (* _returnvalue_4 2.5) false false)
      (return false))))