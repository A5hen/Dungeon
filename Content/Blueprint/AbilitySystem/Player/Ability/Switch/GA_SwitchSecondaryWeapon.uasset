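; Gameplay ability that switches the player's equipped secondary weapon to the next of three slots.
; On activation it commits only the cooldown, reads the current slot from the avatar through a message call and increments it, wrapping back to the first after the third.
; It sends the new slot back to the avatar, opens the equipment panel through the equipped widget controller, then ends immediately.
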(event `self.K2_ActivateAbility`
  (`self.K2_CommitAbilityCooldown` false)
  (bind _returnvalue (message `PlayerInterface.GetCurrentEquippedSecondaryWeaponSlot` (`self.GetAvatarActorFromActorInfo`)))
  (bind _returnvalue_2 (+ _returnvalue 1))
  (if (> _returnvalue_2 3)
    (set `self.NextSlot` 1)
    (else
      (set `self.NextSlot` _returnvalue_2)))
  (message `PlayerInterface.ChangeCurrentEquippedSecondaryWeaponSlot` (`self.GetAvatarActorFromActorInfo`) (`self.NextSlot`))
  (`EquippedWidgetController.OpenEquipmentPanel` (`DungeonAbilitySystemLibrary.GetEquippedWidgetController` null))
  (`self.K2_EndAbility`))