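; Passive player ability that lets the avatar equip or pack a selected pickup item.
; An async input task reports selection changes, each clearing earlier waits; a selection then waits for Input.Async.F to pack, plus Input.Async.R if directly usable.
; Avatar messages check equip eligibility or backpack space, then receive the item info before the pickup is destroyed.
; An interact montage follows, then line tracing re-enables after a short delay.
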(event `self.K2_ActivateAbility`
  (bind (_asynctaskproxy _pickupitem _busedirectly _bselected) (`AsyncInputTask.CreateUAsyncInputTask`)
    (:`OnAsyncInput`
      (`self.ClearAsyncAction`)
      (bind _output_get (set `self.Selected` _bselected))
      (if _output_get
        (set `self.Pickup Item` _pickupitem)
        (set `self.Use Directly` _busedirectly)
        (bind _asbp_pickup_item_base (cast `/Game/Blueprint/Actor/PickupActor/BP_PickupItemBase` (`self.Pickup Item`)))
        (bind _output_get_2 (set `self.BP Pickup Item` _asbp_pickup_item_base))
        (if (`self.Use Directly`)
          (`|ExecutionSequence`
            (:`then_0`
              (bind _asynctaskproxy_2 (`AbilityAsync_WaitGameplayEvent.WaitGameplayEventToActor` (`self.GetAvatarActorFromActorInfo`) (struct :`TagName` "Input.Async.R"))
                (:`then`
                  (set `self.UseAsyncAction` _asynctaskproxy_2))
                (:`EventReceived`
                  (bind _returnvalue (message `PlayerInterface.CanEquip` (`self.GetAvatarActorFromActorInfo`) (`.HandheldType` (break `GameItemInfo` (`PickupItems.ItemInfo` (`self.BP Pickup Item`))))))
                  (if _returnvalue
                    (bind _successfullyuse (`self.UseItemDirectly`))
                    (if _successfullyuse
                      (`AbilityTask_PlayMontageAndWait.CreatePlayMontageAndWaitProxy` "None" "/Game/Asset/Character/Knight/Interact_Montage.Interact_Montage"
                        (:`OnCompleted`
                          _)
                        (:`OnBlendOut`
                          _)
                        (:`OnInterrupted`
                          _))
                      (`AbilityTask_WaitDelay.WaitDelay` 0.1
                        (:`OnFinish`
                          (message `PlayerInterface.SetLineTrace` (`self.GetAvatarActorFromActorInfo`) true))))
                    (else
                      (`KismetSystemLibrary.PrintString` "Can't Equip!!!"))))))
            (:`then_1`
              (bind _asynctaskproxy_3 (`AbilityAsync_WaitGameplayEvent.WaitGameplayEventToActor` (`self.GetAvatarActorFromActorInfo`) (struct :`TagName` "Input.Async.F"))
                (:`then`
                  (set `self.PackAsyncAction` _asynctaskproxy_3))
                (:`EventReceived`
                  (bind _returnvalue_2 (message `PlayerInterface.CheckBackpackIsFull` (`self.GetAvatarActorFromActorInfo`)))
                  (if _returnvalue_2
                    (`KismetSystemLibrary.PrintString` "Can't Equip!!!")
                    (else
                      (`self.PackItem`)
                      (`AbilityTask_PlayMontageAndWait.CreatePlayMontageAndWaitProxy` "None" "/Game/Asset/Character/Knight/Interact_Montage.Interact_Montage"
                        (:`OnCompleted`
                          _)
                        (:`OnBlendOut`
                          _)
                        (:`OnInterrupted`
                          _))
                      (`AbilityTask_WaitDelay.WaitDelay` 0.1
                        (:`OnFinish`
                          (message `PlayerInterface.SetLineTrace` (`self.GetAvatarActorFromActorInfo`) true)))))))))
          (else
            (bind _asynctaskproxy_4 (`AbilityAsync_WaitGameplayEvent.WaitGameplayEventToActor` (`self.GetAvatarActorFromActorInfo`) (struct :`TagName` "Input.Async.F"))
              (:`then`
                (set `self.PackAsyncAction` _asynctaskproxy_4))
              (:`EventReceived`
                (bind _returnvalue_3 (message `PlayerInterface.CheckBackpackIsFull` (`self.GetAvatarActorFromActorInfo`)))
                (if _returnvalue_3
                  (`KismetSystemLibrary.PrintString` "Can't Equip!!!")
                  (else
                    (`self.PackItem`)
                    (`AbilityTask_PlayMontageAndWait.CreatePlayMontageAndWaitProxy` "None" "/Game/Asset/Character/Knight/Interact_Montage.Interact_Montage"
                      (:`OnCompleted`
                        _)
                      (:`OnBlendOut`
                        _)
                      (:`OnInterrupted`
                        _))
                    (`AbilityTask_WaitDelay.WaitDelay` 0.1
                      (:`OnFinish`
                        (message `PlayerInterface.SetLineTrace` (`self.GetAvatarActorFromActorInfo`) true)))))))))))))

(fn `ClearAsyncAction`
  (`/Engine/EditorBlueprintResources/StandardMacros.IsValid` (`self.UseAsyncAction`)
    (:`Is Valid`
      (`AbilityAsync.EndAction` (`self.UseAsyncAction`)))
    (:`Is Not Valid`
      _))
  (`/Engine/EditorBlueprintResources/StandardMacros.IsValid` (`self.PackAsyncAction`)
    (:`Is Valid`
      (`AbilityAsync.EndAction` (`self.PackAsyncAction`)))))

(fn `PackItem`
  (bind _bp_pickup_item (`self.BP Pickup Item`))
  (message `PlayerInterface.AddToBackpack` (`self.GetAvatarActorFromActorInfo`) (`PickupItems.ItemInfo` (`self.BP Pickup Item`)))
  (`/Engine/EditorBlueprintResources/StandardMacros.IsValid` _bp_pickup_item
    (:`Is Valid`
      (`Actor.K2_DestroyActor` _bp_pickup_item))))

(fn `UseItemDirectly`
  (returns (SuccessfullyUse :type Boolean))
  (bind _bp_pickup_item (`self.BP Pickup Item`))
  (bind _returnvalue (message `CharacterInterface.Use` (`self.GetAvatarActorFromActorInfo`) (`PickupItems.ItemInfo` (`self.BP Pickup Item`))))
  (if _returnvalue
    (`/Engine/EditorBlueprintResources/StandardMacros.IsValid` _bp_pickup_item
      (:`Is Valid`
        (`Actor.K2_DestroyActor` _bp_pickup_item)
        (return true))
      (:`Is Not Valid`
        _)))
  (return false))