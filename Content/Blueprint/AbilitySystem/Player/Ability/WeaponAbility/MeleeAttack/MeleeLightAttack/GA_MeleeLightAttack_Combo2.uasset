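; Gameplay ability for the second hit of the player's melee light attack combo.
; On activation it looks up the equipped weapon's info by index, flags the avatar as attacking, and commits a cost set from the weapon's handheld type.
; It plays the weapon's combo-2 montage from the count-to-montage map and ends when that montage completes, blends out or is interrupted.
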(event `self.K2_ActivateAbility`
  (`self.GetCurrentEquipedWeaponInfo`)
  (message `PlayerInterface.SetIsAttacking` (`self.GetAvatarActorFromActorInfo`) true)
  (`self.Cost`)
  (`AbilityTask_PlayMontageAndWait.CreatePlayMontageAndWaitProxy` "None" (`BlueprintMapLibrary.Map_Find` (`self.Count To Montage`) 2) 1.0 "None" false
    (:`OnCompleted`
      _)
    (:`OnBlendOut`
      _)
    (:`OnInterrupted`
      _))
  (`self.K2_EndAbility`))

(fn `Cost`
  (bind _returnvalue (message `PlayerInterface.GetEquipedWeaponInfo` (`self.GetAvatarActorFromActorInfo`)))
  (`self.SetCost` (`.HandheldType` (break `GameItemInfo` _returnvalue)))
  (`self.K2_CommitAbilityCost` false))

(fn `GetCurrentEquipedWeaponInfo`
  (bind _returnvalue (message `CharacterInterface.GetWeaponIndex` (`self.GetAvatarActorFromActorInfo`)))
  (set `self.EquipedWeaponIndex` _returnvalue)
  (bind _returnvalue_2 (`DungeonAbilitySystemLibrary.GetEquipmentInfomation` null))
  (bind _returnvalue_3 (`DetailedEquipmemtInfo.GetWeaponInfoForItemIndex` _returnvalue_2 (`self.EquipedWeaponIndex`)))
  (set `self.Count To Montage` (`.CountToMontage` (break `WeaponInfo` _returnvalue_3))))