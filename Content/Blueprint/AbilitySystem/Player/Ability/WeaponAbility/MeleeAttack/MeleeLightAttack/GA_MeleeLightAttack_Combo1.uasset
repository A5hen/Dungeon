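; Gameplay Ability for the first hit of the player's melee light attack combo.
; On activation it looks up the equipped weapon's montage map by weapon index, flags the avatar as attacking and takes the entry for count 1.
; With a valid montage, it commits a cost based on the weapon's handheld type and plays it, ending on completion, blend out or interruption.
; Without one, it clears the attacking flag and ends.
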(event `self.K2_ActivateAbility`
  (bind _value (`BlueprintMapLibrary.Map_Find` (`self.Count To Montage`) 1))
  (`self.GetCurrentEquipedWeaponInfo`)
  (message `PlayerInterface.SetIsAttacking` (`self.GetAvatarActorFromActorInfo`) true)
  (`/Engine/EditorBlueprintResources/StandardMacros.IsValid` _value
    (:`Is Valid`
      (`self.Cost`)
      (`AbilityTask_PlayMontageAndWait.CreatePlayMontageAndWaitProxy` "None" _value 1.0 "None" false
        (:`OnCompleted`
          _)
        (:`OnBlendOut`
          _)
        (:`OnInterrupted`
          _))
      (`self.K2_EndAbility`))
    (:`Is Not Valid`
      (message `PlayerInterface.SetIsAttacking` (`self.GetAvatarActorFromActorInfo`) false)
      (`self.K2_EndAbility`))))

(fn `Cost`
  (bind _returnvalue (message `PlayerInterface.GetEquipedWeaponInfo` (`self.GetAvatarActorFromActorInfo`)))
  (`self.SetCost` (`.HandheldType` (break `GameItemInfo` _returnvalue)))
  (`self.K2_CommitAbilityCost` false))

(fn `GetCurrentEquipedWeaponInfo`
  (bind _returnvalue (message `CharacterInterface.GetWeaponIndex` (`self.GetAvatarActorFromActorInfo`)))
  (set `self.EquipedWeaponIndex` _returnvalue)
  (bind _returnvalue_2 (`DungeonAbilitySystemLibrary.GetEquipmentInfomation` null))
  (bind _returnvalue_3 (`DetailedEquipmemtInfo.GetWeaponInfoForItemIndex` _returnvalue_2 (`self.EquipedWeaponIndex`)))
  (set `self.Count To Montage` (`.CountToMontage` (break `WeaponInfo` _returnvalue_3))))