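; Gameplay ability that picks and triggers the next melee combo step for the avatar's equipped weapon.
; On activation it selects a one-handed or two-handed tag list from the weapon's handheld type, defaulting to one-handed, and exits if already attacking.
; It finds the active combo tag on the ability system and sends the following tag as a gameplay event, restarting at the first combo when none matches or the chain ends.
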(event `self.K2_ActivateAbility`
  (`self.SetComboByType`)
  (bind _returnvalue (message `PlayerInterface.GetIsAttacking` (`self.GetAvatarActorFromActorInfo`)))
  (if (not _returnvalue)
    (for (_array_element _array_index) (`self.ComboTag`)
      (set `self.Array Index` _array_index)
      (if (`GameplayTagAssetInterface.HasMatchingGameplayTag` (`self.GetAbilitySystemComponentFromActorInfo`) _array_element)
        (if (not (`self.AlreadyTakeAction`))
          (if (< (+ (`self.Array Index`) 1) (`KismetArrayLibrary.Array_Length` (`self.ComboTag`)))
            (`AbilitySystemBlueprintLibrary.SendGameplayEventToActor` (`self.GetAvatarActorFromActorInfo`) (`|GetArrayItem` (`self.ComboTag`) (+ (`self.Array Index`) 1)))
            (set `self.AlreadyTakeAction` true)
            (else
              (`AbilitySystemBlueprintLibrary.SendGameplayEventToActor` (`self.GetAvatarActorFromActorInfo`) (struct :`TagName` "MeleeAbility.Combo.1"))
              (set `self.AlreadyTakeAction` true))))))
    (if (`GameplayTagAssetInterface.HasAnyMatchingGameplayTags` (`self.GetAbilitySystemComponentFromActorInfo`) (`BlueprintGameplayTagLibrary.MakeGameplayTagContainerFromArray` (`self.ComboTag`)))
      (set `self.AlreadyTakeAction` false)
      (`self.K2_EndAbility`)
      (else
        (`AbilitySystemBlueprintLibrary.SendGameplayEventToActor` (`self.GetAvatarActorFromActorInfo`) (struct :`TagName` "MeleeAbility.Combo.1"))
        (set `self.AlreadyTakeAction` false)
        (`self.K2_EndAbility`)))
    (else
      (`self.K2_EndAbility`))))

(fn `SetComboByType`
  (bind _returnvalue (message `PlayerInterface.GetEquipedWeaponInfo` (`self.GetAvatarActorFromActorInfo`)))
  (bind (_itemindex _itemtype _handheldtype) (break `GameItemInfo` _returnvalue))
  (if (== _handheldtype (struct :`TagName` "Handheld.1H"))
    (set `self.ComboTag` (`self.1HTag`))
    (elif (== _handheldtype (struct :`TagName` "Handheld.2H"))
      (set `self.ComboTag` (`self.2HTag`))
      (else
        (set `self.ComboTag` (`self.1HTag`))))))