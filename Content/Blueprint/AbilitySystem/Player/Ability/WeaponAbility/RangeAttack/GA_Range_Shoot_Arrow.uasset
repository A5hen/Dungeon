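; Gameplay ability that fires an arrow from the player's ranged weapon, or reloads it when unloaded.
; If loaded, it plays a one- or two-handed shoot montage, commits cost, and on the Montage.Shoot event spawns a pitch-overridden arrow using aim and lock-on state, then unloads.
; Otherwise, if loading is allowed, it plays a reload montage that marks the weapon loaded unless interrupted.
; Weapon state flows through message calls on the avatar.
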(event `self.K2_ActivateAbility`
  (set `self.Actor` (`self.GetAvatarActorFromActorInfo`))
  (bind _returnvalue (message `PlayerInterface.GetIsLoaded` (`self.Actor`)))
  (if _returnvalue
    (`AbilityTask_PlayMontageAndWait.CreatePlayMontageAndWaitProxy` "None" (`self.GetShootMontage`)
      (:`then`
        (`AbilityAsync_WaitGameplayEvent.WaitGameplayEventToActor` (`self.Actor`) (struct :`TagName` "Montage.Shoot") true
          (:`then`
            (`self.K2_CommitAbilityCost` false))
          (:`EventReceived`
            (bind _returnvalue_2 (message `PlayerInterface.GetIsAiming` (`self.Actor`)))
            (bind _returnvalue_3 (message `PlayerInterface.GetIsLocking` (`self.Actor`)))
            (`self.SpawnProjectile` _returnvalue_2 _returnvalue_3 true 15.0 true)
            (message `PlayerInterface.SetIsLoaded` (`self.Actor`) false))))
      (:`OnCompleted`
        (`self.K2_EndAbility` :!label _label))
      (:`OnBlendOut`
        (goto _label))
      (:`OnInterrupted`
        (goto _label)))
    (else
      (bind _returnvalue_4 (message `PlayerInterface.CanLoad` (`self.Actor`)))
      (if _returnvalue_4
        (`AbilityTask_PlayMontageAndWait.CreatePlayMontageAndWaitProxy` "None" "/Game/Asset/Character/Knight/1H_Ranged_Reload_Montage.1H_Ranged_Reload_Montage"
          (:`OnCompleted`
            (message `PlayerInterface.SetIsLoaded` (`self.Actor`) true :!label _label_2))
          (:`OnBlendOut`
            (goto _label_2))
          (:`OnInterrupted`
            _))
        (`self.K2_EndAbility`)
        (else
          (`self.K2_EndAbility`))))))

(fn `GetShootMontage`
  (returns (ShootMontage :type "AnimMontage Object Reference"))
  (bind _returnvalue (message `CharacterInterface.GetEHandheldType` (`self.Actor`)))
  (if (`|EnumEquality` _returnvalue "OneHand")
    (return "/Game/Asset/Character/Knight/1H_Ranged_Shoot_Montage_Kight.1H_Ranged_Shoot_Montage_Kight")
    (else
      (return "/Game/Asset/Character/Knight/2H_Ranged_Shoot_Montage.2H_Ranged_Shoot_Montage"))))