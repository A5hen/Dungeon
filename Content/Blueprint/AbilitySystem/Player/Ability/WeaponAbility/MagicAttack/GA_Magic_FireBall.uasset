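; Player magic ability that casts a fireball projectile.
; If the avatar has the Ability.Enhance tag, it consumes the tag and switches to the enhanced projectile and long spellcast montage.
; The montage's MagicEffect gameplay event commits the cost and spawns the projectile, passing the avatar's lock-on state.
; The ability ends when the montage completes, blends out or is interrupted.
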(event `self.K2_ActivateAbility`
  (if (`GameplayTagAssetInterface.HasMatchingGameplayTag` (`self.GetAbilitySystemComponentFromActorInfo`) (struct :`TagName` "Ability.Enhance"))
    (`AbilitySystemBlueprintLibrary.RemoveLooseGameplayTags` (`self.GetAvatarActorFromActorInfo`) (`BlueprintGameplayTagLibrary.MakeLiteralGameplayTagContainer` (struct :`GameplayTags` (struct :`(TagName` "Ability.Enhance")))))
    (set `self.ProjectileClass` "/Game/Blueprint/Actor/Projectile/BP_Projectile_FireBall_Enhanced.BP_Projectile_FireBall_Enhanced_C")
    (set `self.Montage to Play` "/Game/Asset/Character/Knight/Spellcast_Long_Montage.Spellcast_Long_Montage"))
  (`AbilityTask_PlayMontageAndWait.CreatePlayMontageAndWaitProxy` "None" (`self.Montage to Play`) 1.0 "None" false
    (:`then`
      (`AbilityAsync_WaitGameplayEvent.WaitGameplayEventToActor` (`self.GetAvatarActorFromActorInfo`) (struct :`TagName` "Montage.MagicEffect") true
        (:`EventReceived`
          (`self.K2_CommitAbilityCost` false)
          (bind _returnvalue (message `PlayerInterface.GetIsLocking` (`self.GetAvatarActorFromActorInfo`)))
          (`self.SpawnProjectile` false _returnvalue))))
    (:`OnCompleted`
      (`self.K2_EndAbility` :!label _label))
    (:`OnBlendOut`
      (goto _label))
    (:`OnInterrupted`
      (goto _label))))