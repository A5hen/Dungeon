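; Gameplay ability for the secondary-weapon shield, active while its input is held and offering a block attack.
; On activation it waits for input release, binds to the character's blocking-end event to end itself, and listens for the LM input.
; LM plays the block attack montage unless the equipped weapon is two-handed.
; Release ends the ability unless that attack has started, in which case montage completion, blend-out or interruption ends it.
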(event `OnBlockingEnd_事件`
  (`self.K2_EndAbility`))

(event `self.K2_ActivateAbility`
  (`AbilityTask_WaitInputRelease.WaitInputRelease` false
    (:`then`
      (bind _ascharacter_base (cast `CharacterBase` (`self.GetAvatarActorFromActorInfo`)))
      (add `CharacterBase.OnBlockingEnd` _ascharacter_base (delegate `OnBlockingEnd_事件`))
      (`SpecificInputTask.CreateUSpecificInputTask` (`self.LM`)
        (:`OnSpecificInput`
          (bind _returnvalue (message `PlayerInterface.GetEquipedWeaponInfo` (`self.GetAvatarActorFromActorInfo`)))
          (if (!= (`.ItemType` (break `GameItemInfo` _returnvalue)) (struct :`TagName` "Handheld.2H"))
            (set `self.IsBlockAttack` true)
            (`AbilityTask_PlayMontageAndWait.CreatePlayMontageAndWaitProxy` "None" "/Game/Asset/Character/Knight/Block_Attack_Montage.Block_Attack_Montage"
              (:`OnCompleted`
                _)
              (:`OnBlendOut`
                _)
              (:`OnInterrupted`
                _))
            (`self.K2_EndAbility`)))))
    (:`OnRelease`
      (if (not (`self.IsBlockAttack`))
        (`self.K2_EndAbility`)))))