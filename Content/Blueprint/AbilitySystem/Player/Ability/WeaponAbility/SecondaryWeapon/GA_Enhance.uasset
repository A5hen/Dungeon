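; Gameplay ability for a secondary weapon that applies an Enhance state to the player.
; It ends early if secondary durability is zero, the current weapon type is not Magic, or the Ability.Enhance tag is already present.
; Otherwise it commits cost, spends secondary durability and plays a spellcast montage.
; On completion, blend-out or interruption, it adds the non-replicated loose Ability.Enhance tag and ends.
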(event `self.K2_ActivateAbility`
  (set `self.Actor` (`self.GetAvatarActorFromActorInfo`))
  (bind _returnvalue (message `CharacterInterface.GetDurability` (`self.Actor`) true))
  (if (== _returnvalue 0.0)
    (`self.K2_EndAbility`)
    (else
      (bind _returnvalue_2 (message `CharacterInterface.GetCurrentWeaponType` (`self.Actor`)))
      (if (== _returnvalue_2 (struct :`TagName` "Weapon.Magic"))
        (if (`GameplayTagAssetInterface.HasMatchingGameplayTag` (`self.GetAbilitySystemComponentFromActorInfo`) (struct :`TagName` "Ability.Enhance"))
          (`self.K2_EndAbility`)
          (else
            (`self.K2_CommitAbilityCost` false)
            (message `CharacterInterface.SetDurability` (`self.Actor`) -1.0 true)
            (`AbilityTask_PlayMontageAndWait.CreatePlayMontageAndWaitProxy` "None" "/Game/Asset/Character/Knight/Spellcast_Raise_Montage.Spellcast_Raise_Montage"
              (:`OnCompleted`
                _)
              (:`OnBlendOut`
                _)
              (:`OnInterrupted`
                _))
            (`AbilitySystemBlueprintLibrary.AddLooseGameplayTags` (`self.Actor`) (`BlueprintGameplayTagLibrary.MakeLiteralGameplayTagContainer` (struct :`GameplayTags` (struct :`(TagName` "Ability.Enhance")))))
            (`self.K2_EndAbility`)))
        (else
          (`self.K2_EndAbility`))))))