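; GA_TraceCheck is a player combat Gameplay Ability that runs weapon-trace hit detection.
; On activation it gets the avatar's weapon mesh, primes the trace and starts a looping timer at the current frame's delta time.
; Each tick traces along the weapon, applies effects to hit actors, then either prepares the next trace or, if blocked, sends Ability.Interrupt and ends.
; The character's OnTraceCheckEnd callback also stops the timer and ends the ability.
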(event `OnTraceCheckEnd_事件`
  (bind _timerhandle (`self.TimerHandle`))
  (if (`KismetSystemLibrary.K2_IsValidTimerHandle` _timerhandle)
    (`KismetSystemLibrary.K2_ClearAndInvalidateTimerHandle` _timerhandle)
    (`self.K2_EndAbility`)
    (else
      (`self.K2_EndAbility`))))

(event `self.K2_ActivateAbility`
  (bind _returnvalue (message `CharacterInterface.GetWeaponStaticMeshComponent` (`self.GetAvatarActorFromActorInfo`)))
  (bind _output_get (set `self.Weapon` _returnvalue))
  (`self.PreTraceCheck` _output_get)
  (bind _returnvalue_2 (`KismetSystemLibrary.K2_SetTimerDelegate` (delegate `Timer`) (`GameplayStatics.GetWorldDeltaSeconds`) true))
  (set `self.TimerHandle` _returnvalue_2)
  (bind _ascharacter_base (cast `CharacterBase` (`self.GetAvatarActorFromActorInfo`))
    (:`then`
      (add `CharacterBase.OnTraceCheckEnd` _ascharacter_base (delegate `OnTraceCheckEnd_事件`)))
    (:`CastFailed`
      (`self.K2_EndAbility`))))

(event `Timer`
  (`KismetArrayLibrary.Array_Clear` (`self.TraceLineActors`))
  (bind _outs (`self.TraceCheckTimerFunction` (`self.TraceLineActors`) (`|MakeArray` (`self.GetAvatarActorFromActorInfo`)) 3.0 (`self.Weapon`)))
  (for _array_element _outs
    (bind _output_get (set `self.TargetActor` _array_element))
    (`self.ApplyEffectInOneRound` _output_get))
  (if (`self.bBlocked`)
    (`AbilitySystemBlueprintLibrary.SendGameplayEventToActor` (`self.GetAvatarActorFromActorInfo`) (struct :`TagName` "Ability.Interrupt"))
    (`KismetSystemLibrary.K2_ClearAndInvalidateTimerHandle` (`self.TimerHandle`))
    (`self.K2_EndAbility`)
    (else
      (`self.PrepareForNext` (`self.Weapon`)))))