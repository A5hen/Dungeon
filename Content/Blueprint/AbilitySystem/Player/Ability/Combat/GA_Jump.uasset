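; Player jump Gameplay Ability with hold-to-jump-higher control, which ends at once if the avatar is already falling.
; A per-frame looping timer adds upward velocity impulses until input release or a time cap, with a minimum hold delay for quick taps.
; A Montage.Land event stops the timer, broadcasts spinning and trace-check end messages, plays a landing montage when its magnitude is one, then commits cooldown and ends.
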(event `Jump`
  (bind _returnvalue (message `PlayerInterface.GetCharacterMovementComponent` (`self.GetAvatarActorFromActorInfo`)))
  (`CharacterMovementComponent.AddImpulse` _returnvalue (0.0 0.0 30.0) true)
  (bind _output_get (set `self.HeldTime` (+ (`self.HeldTime`) (`GameplayStatics.GetWorldDeltaSeconds`))))
  (if (> _output_get 0.16)
    (`KismetSystemLibrary.K2_ClearAndInvalidateTimerHandle` (`self.JumpHandle`))))

(event `self.K2_ActivateAbility`
  (bind _returnvalue (`self.GetAvatarActorFromActorInfo`))
  (bind _returnvalue_2 (`self.GetAvatarActorFromActorInfo`))
  (bind _returnvalue_3 (message `CharacterInterface.GetIsFalling` (`self.GetAvatarActorFromActorInfo`)))
  (if _returnvalue_3
    (`self.K2_EndAbility`)
    (else
      (`self.K2_CommitAbilityCost` false)
      (set `self.HeldTime` 0.0)
      (`|ExecutionSequence`
        (:`then_0`
          (`AbilityTask_WaitInputRelease.WaitInputRelease` false
            (:`then`
              (bind _returnvalue_4 (`KismetSystemLibrary.K2_SetTimerDelegate` (delegate `Jump`) (`GameplayStatics.GetWorldDeltaSeconds`) true))
              (set `self.JumpHandle` _returnvalue_4))
            (:`OnRelease`
              (if (< (`self.HeldTime`) 0.12)
                (`KismetSystemLibrary.Delay` (- 0.12 (`self.HeldTime`))))
              (`KismetSystemLibrary.K2_ClearAndInvalidateTimerHandle` (`self.JumpHandle`)))))
        (:`then_1`
          (bind (_asynctaskproxy _payload) (`AbilityAsync_WaitGameplayEvent.WaitGameplayEventToActor` (`self.GetAvatarActorFromActorInfo`) (struct :`TagName` "Montage.Land") true)
            (:`EventReceived`
              (if (== (`.EventMagnitude` (break `GameplayEventData` _payload)) 1.0)
                (`AbilityTask_PlayMontageAndWait.CreatePlayMontageAndWaitProxy` "None" "/Game/Asset/Character/Knight/Jump_Land_Montage.Jump_Land_Montage" 1.0 "None" false
                  (:`then`
                    (message `CharacterInterface.BroadcastSpinningEndDelegate` _returnvalue_2)
                    (message `CharacterInterface.BroadcastTraceCheckEndDelegate` _returnvalue_2)
                    (`KismetSystemLibrary.K2_ClearAndInvalidateTimerHandle` (`self.JumpHandle`)))
                  (:`OnCompleted`
                    (`self.K2_CommitAbilityCooldown` false :!label _label)
                    (`self.K2_EndAbility`))
                  (:`OnBlendOut`
                    (goto _label))
                  (:`OnInterrupted`
                    (goto _label)))
                (else
                  (message `CharacterInterface.BroadcastSpinningEndDelegate` _returnvalue)
                  (message `CharacterInterface.BroadcastTraceCheckEndDelegate` _returnvalue)
                  (`KismetSystemLibrary.K2_ClearAndInvalidateTimerHandle` (`self.JumpHandle`))
                  (`self.K2_CommitAbilityCooldown` false)
                  (`self.K2_EndAbility`))))))))))