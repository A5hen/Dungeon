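; Gameplay ability that toggles target lock-on for the avatar, ending immediately after each activation.
; When unlocked, it finds the closest in-sight character with the opposing Player or Enemy tag and locks onto it if valid.
; Locking switches movement to controller-facing rotation, shifts the spring arm offset and hides the aux spline; unlocking restores movement orientation and camera offset.
; Avatar state is accessed through message calls, with no casting.
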(event `self.K2_ActivateAbility`
  (bind _avataractor (`self.AvatarActor`))
  (set `self.AvatarActor` (`self.GetAvatarActorFromActorInfo`))
  (bind _returnvalue (message `PlayerInterface.GetIsLocking` (`self.AvatarActor`)))
  (if _returnvalue
    (message `PlayerInterface.SetIsLocking` (`self.AvatarActor`) false)
    (`self.SetMoveComponent` false)
    (message `PlayerInterface.SetSpringArmOffset` (`self.AvatarActor`) 0.0 0.0 35.0)
    (`self.K2_EndAbility`)
    (else
      (bind _outactor (`DungeonAbilitySystemLibrary.GetClosestCharacterInSightByTag` null (`|MakeArray` _avataractor) 1000.0 (`Actor.K2_GetActorLocation` _avataractor) (`self.GetTargetTag`)))
      (bind _output_get (set `self.TargetActor` _outactor))
      (`/Engine/EditorBlueprintResources/StandardMacros.IsValid` _output_get
        (:`Is Valid`
          (message `CharacterInterface.SetTargetActor` (`self.AvatarActor`) (`self.TargetActor`))
          (message `PlayerInterface.SetIsLocking` (`self.AvatarActor`) true)
          (`self.SetMoveComponent` true)
          (message `PlayerInterface.SetSpringArmOffset` (`self.AvatarActor`) -20.0 0.0 50.0)
          (message `PlayerInterface.EndShowAuxSpline` (`self.AvatarActor`))
          (`self.K2_EndAbility`))
        (:`Is Not Valid`
          (`self.K2_EndAbility`))))))

(fn `GetTargetTag`
  (returns (TargetTag :type "GameplayTag Structure"))
  (locals (OwnerTag :type "GameplayTag Structure"))
  (bind _returnvalue (message `CharacterInterface.GetCharacterTag` (`self.GetAvatarActorFromActorInfo`)))
  (set `local.OwnerTag` _returnvalue)
  (if (== (`local.OwnerTag`) (struct :`TagName` "Character.Player"))
    (return (struct :`TagName` "Character.Enemy"))
    (elif (== (`local.OwnerTag`) (struct :`TagName` "Character.Enemy"))
      (return (struct :`TagName` "Character.Player"))
      (else
        (return)))))

(fn `SetMoveComponent`
  (params (bLock :type Boolean))
  (locals (InBool :type Boolean))
  (set `local.InBool` bLock)
  (bind _returnvalue (message `PlayerInterface.GetCharacterMovementComponent` (`self.AvatarActor`)))
  (set `CharacterMovementComponent.bUseControllerDesiredRotation` (`local.InBool`) _returnvalue)
  (set `CharacterMovementComponent.bOrientRotationToMovement` (not (`local.InBool`)) _returnvalue))