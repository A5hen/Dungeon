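; Player gameplay ability for aiming and throwing the current one-handed weapon.
; Activation drops lock-on and shows an aim spline with controller-driven yaw, while input tasks switch throw angle or cancel.
; Releasing input plays the throw montage; its Montage.Throw event or an interruption commits cost, throws and uses the current consumable.
; All endings, cancellation included, run EndThrow, which clears aim state and commits cooldown.
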(event `self.K2_ActivateAbility`
  (set `self.AvatarActor` (`self.GetAvatarActorFromActorInfo`))
  (`self.EndLock`)
  (`AbilityTask_WaitInputRelease.WaitInputRelease` false
    (:`then`
      (message `PlayerInterface.SetShowAuxSpline` (`self.AvatarActor`) true)
      (message `PlayerInterface.SetUseControllerRotationYaw` (`self.AvatarActor`) true)
      (bind _asynctaskproxy (`SpecificInputTask.CreateUSpecificInputTask` (`self.EndTag`))
        (:`then`
          (set `self.End Task` _asynctaskproxy)
          (bind _asynctaskproxy_2 (`SpecificInputTask.CreateUSpecificInputTask` (`self.SwitchTag`))
            (:`then`
              (set `self.SwitchTask` _asynctaskproxy_2))
            (:`OnSpecificInput`
              (message `PlayerInterface.SwitchThrowAngle` (`self.AvatarActor`)))))
        (:`OnSpecificInput`
          (`self.EndThrow`))))
    (:`OnRelease`
      (`AbilityTask_PlayMontageAndWait.CreatePlayMontageAndWaitProxy` "None" "/Game/Asset/Character/Knight/Throw_Montage.Throw_Montage" 1.0 "None" false
        (:`then`
          (message `PlayerInterface.SetShowAuxSpline` (`self.AvatarActor`) false)
          (message `PlayerInterface.EndShowAuxSpline` (`self.AvatarActor`))
          (`AbilityAsync_WaitGameplayEvent.WaitGameplayEventToActor` (`self.AvatarActor`) (struct :`TagName` "Montage.Throw") true
            (:`EventReceived`
              (`self.K2_CommitAbilityCost` false :!label _label)
              (`self.ThrowCurrentWeapon_1H`)
              (message `PlayerInterface.UseCurrentConsumable` (`self.AvatarActor`))
              (`self.EndThrow`))))
        (:`OnCompleted`
          (`self.EndThrow` :!label _label_2))
        (:`OnBlendOut`
          (goto _label_2))
        (:`OnInterrupted`
          (goto _label))))))

(fn `EndLock`
  (message `PlayerInterface.SetIsLocking` (`self.GetAvatarActorFromActorInfo`) false)
  (bind _returnvalue (message `PlayerInterface.GetCharacterMovementComponent` (`self.GetAvatarActorFromActorInfo`)))
  (set `CharacterMovementComponent.bUseControllerDesiredRotation` false _returnvalue)
  (set `CharacterMovementComponent.bOrientRotationToMovement` true _returnvalue)
  (message `PlayerInterface.SetSpringArmOffset` (`self.GetAvatarActorFromActorInfo`) 0.0 0.0 35.0))

(fn `EndThrow`
  (bind _avataractor (`self.AvatarActor`))
  (message `PlayerInterface.SetShowAuxSpline` _avataractor false)
  (message `PlayerInterface.EndShowAuxSpline` _avataractor)
  (message `PlayerInterface.SetUseControllerRotationYaw` (`self.AvatarActor`) false)
  (bind _end_task (`self.End Task`)
    (:`then`
      (`GameplayTask.EndTask` _end_task))
    (:`else`
      _))
  (bind _switchtask (`self.SwitchTask`)
    (:`then`
      (`GameplayTask.EndTask` _switchtask))
    (:`else`
      _))
  (`self.K2_CommitAbilityCooldown` false)
  (`self.K2_EndAbility`))