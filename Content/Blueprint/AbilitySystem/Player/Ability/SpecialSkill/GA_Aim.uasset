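; Player gameplay ability that toggles aiming while the current weapon is exactly a ranged weapon.
; Entering aim sets the aiming flag, applies GE_AimEffect and cancels target lock, restoring movement-oriented rotation and the spring arm offset.
; Leaving aim clears the flag and removes effects granting RangeAbility.Aim.
; Avatar state is accessed through message calls, and the ability ends itself after a short delay in every branch.
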(event `self.K2_ActivateAbility`
  (bind _returnvalue (`self.GetAbilitySystemComponentFromActorInfo`))
  (bind _returnvalue_2 (message `CharacterInterface.GetCurrentWeaponType` (`self.GetAvatarActorFromActorInfo`)))
  (if (`BlueprintGameplayTagLibrary.MatchesTag` _returnvalue_2 (struct :`TagName` "Weapon.Range") true)
    (bind _returnvalue_3 (message `PlayerInterface.GetIsAiming` (`self.GetAvatarActorFromActorInfo`)))
    (if _returnvalue_3
      (message `PlayerInterface.SetIsAiming` (`self.GetAvatarActorFromActorInfo`) false)
      (`self.BP_RemoveGameplayEffectFromOwnerWithGrantedTags` (struct :`GameplayTags` (struct :`(TagName` "RangeAbility.Aim"))))
      (`AbilityTask_WaitDelay.WaitDelay` 0.3
        (:`OnFinish`
          (`self.K2_EndAbility`)))
      (else
        (message `PlayerInterface.SetIsAiming` (`self.GetAvatarActorFromActorInfo`) true)
        (`self.K2_ApplyGameplayEffectSpecToOwner` (`AbilitySystemComponent.MakeOutgoingSpec` _returnvalue "/Game/Blueprint/AbilitySystem/Player/Ability/SpecialSkill/GE_AimEffect.GE_AimEffect_C" 1.0 (`AbilitySystemComponent.MakeEffectContext` _returnvalue)))
        (`self.CancelLockTarget`)
        (`AbilityTask_WaitDelay.WaitDelay` 0.3
          (:`OnFinish`
            (`self.K2_EndAbility`)))))
    (else
      (`AbilityTask_WaitDelay.WaitDelay` 0.1
        (:`OnFinish`
          (`self.K2_EndAbility`))))))

(fn `CancelLockTarget`
  (message `PlayerInterface.SetIsLocking` (`self.GetAvatarActorFromActorInfo`) false)
  (bind _returnvalue (message `PlayerInterface.GetCharacterMovementComponent` (`self.GetAvatarActorFromActorInfo`)))
  (set `CharacterMovementComponent.bUseControllerDesiredRotation` false _returnvalue)
  (set `CharacterMovementComponent.bOrientRotationToMovement` true _returnvalue)
  (message `PlayerInterface.SetSpringArmOffset` (`self.GetAvatarActorFromActorInfo`) 0.0 0.0 35.0))