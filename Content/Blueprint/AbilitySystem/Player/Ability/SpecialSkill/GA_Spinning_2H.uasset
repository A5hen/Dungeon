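; Player gameplay ability for a two-handed spinning melee attack held while the input is down.
; A start montage's gameplay event sets the spinning state and starts a looping frame-interval timer that commits the ability cost.
; On input release, it waits for the end-spin montage event, then plays the end montage, clears state and ends.
; The character's OnSpinningEnd delegate also stops the spin and timer and ends the ability directly.
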(event `OnSpinningEnd_事件`
  (message `CharacterInterface.SetIsSpinning` (`self.AvatarActor`) false)
  (message `PlayerInterface.SetUseControllerRotationYaw` (`self.AvatarActor`) false)
  (`KismetSystemLibrary.K2_ClearAndInvalidateTimerHandle` (`self.Timer`))
  (`self.K2_EndAbility`))

(event `self.K2_ActivateAbility`
  (set `self.AvatarActor` (`self.GetAvatarActorFromActorInfo`))
  (`AbilityTask_WaitInputRelease.WaitInputRelease` false
    (:`then`
      (message `PlayerInterface.SetIsAttacking` (`self.AvatarActor`) true)
      (`AbilityTask_PlayMontageAndWait.CreatePlayMontageAndWaitProxy` "None" "/Game/Asset/Character/Knight/2H_Melee_Attack_Spin_Start_Montage.2H_Melee_Attack_Spin_Start_Montage"
        (:`then`
          (message `PlayerInterface.SetUseControllerRotationYaw` (`self.AvatarActor`) true)
          (`AbilityAsync_WaitGameplayEvent.WaitGameplayEventToActor` (`self.AvatarActor`) (struct :`TagName` "Montage.Spinning") true
            (:`then`
              (bind _ascharacter_base (cast `CharacterBase` (`self.AvatarActor`)))
              (add `CharacterBase.OnSpinningEnd` _ascharacter_base (delegate `OnSpinningEnd_事件`)))
            (:`EventReceived`
              (message `CharacterInterface.SetIsSpinning` (`self.AvatarActor`) true)
              (bind _returnvalue (`KismetSystemLibrary.K2_SetTimerDelegate` (delegate `Cost`) (`GameplayStatics.GetWorldDeltaSeconds`) true))
              (set `self.Timer` _returnvalue))))))
    (:`OnRelease`
      (`AbilityAsync_WaitGameplayEvent.WaitGameplayEventToActor` (`self.AvatarActor`) (struct :`TagName` "Montage.EndSpinning") true
        (:`EventReceived`
          (`AbilityTask_PlayMontageAndWait.CreatePlayMontageAndWaitProxy` "None" "/Game/Asset/Character/Knight/2H_Melee_Attack_Spin_End_Montage.2H_Melee_Attack_Spin_End_Montage"
            (:`then`
              (message `CharacterInterface.SetIsSpinning` (`self.AvatarActor`) false)
              (message `PlayerInterface.SetUseControllerRotationYaw` (`self.AvatarActor`) false))
            (:`OnCompleted`
              (message `PlayerInterface.SetIsAttacking` (`self.AvatarActor`) false :!label _label)
              (`KismetSystemLibrary.K2_ClearAndInvalidateTimerHandle` (`self.Timer`))
              (`self.K2_EndAbility`))
            (:`OnBlendOut`
              (goto _label))
            (:`OnInterrupted`
              (goto _label))))))))

(event `Cost`
  (`self.K2_CommitAbilityCost` false))