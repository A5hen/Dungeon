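; Gameplay ability for enemies that plays an awake montage on the avatar and then flags it as awake.
; On activation it asks the avatar for one of two montages by random index, through a message call.
; Completion, blend out or interruption of the montage sets the awake flag and ends the ability.
; With no valid montage, the ability ends without setting the flag.
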(event `self.K2_ActivateAbility`
  (bind _returnvalue (message `EnemyInterface.GetAwakeMontage` (`self.GetAvatarActorFromActorInfo`) (`KismetMathLibrary.RandomIntegerInRange` 0 1)))
  (bind _output_get (set `self.AwakeMontage` _returnvalue))
  (`/Engine/EditorBlueprintResources/StandardMacros.IsValid` _output_get
    (:`Is Valid`
      (`AbilityTask_PlayMontageAndWait.CreatePlayMontageAndWaitProxy` "None" (`self.AwakeMontage`)
        (:`OnCompleted`
          _)
        (:`OnBlendOut`
          _)
        (:`OnInterrupted`
          _))
      (message `EnemyInterface.SetIsAwake` (`self.GetAvatarActorFromActorInfo`) true)
      (`self.K2_EndAbility`))
    (:`Is Not Valid`
      (`self.K2_EndAbility`))))