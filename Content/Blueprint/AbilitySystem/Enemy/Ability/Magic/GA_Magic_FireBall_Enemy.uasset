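; Enemy fireball spell ability that plays a shoot montage and spawns a lock-on projectile on the Montage.MagicEffect gameplay event.
; An Ability.Enhance tag on the caster is consumed to switch to the enhanced fireball class.
; Without the tag, a magic-enhance secondary item with nonzero durability makes the cast a raise montage instead, which adds the tag and spends durability.
; With that item at zero durability, the ability neither fires nor calls EndAbility.
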(event `self.K2_ActivateAbility`
  (set `self.Actor` (`self.GetAvatarActorFromActorInfo`))
  (bind _output_get (set `self.bEnhanced` (`GameplayTagAssetInterface.HasMatchingGameplayTag` (`self.GetAbilitySystemComponentFromActorInfo`) (struct :`TagName` "Ability.Enhance"))))
  (if _output_get
    (`AbilitySystemBlueprintLibrary.RemoveLooseGameplayTags` (`self.Actor`) (`BlueprintGameplayTagLibrary.MakeLiteralGameplayTagContainer` (struct :`GameplayTags` (struct :`(TagName` "Ability.Enhance")))))
    (set `self.ProjectileClass` "/Game/Blueprint/Actor/Projectile/BP_Projectile_FireBall_Enhanced.BP_Projectile_FireBall_Enhanced_C")
    (bind _returnvalue (message `EnemyInterface.GetShootMontage` (`self.Actor`) (`self.bEnhanced`) :!label _label))
    (`AbilityTask_PlayMontageAndWait.CreatePlayMontageAndWaitProxy` "None" _returnvalue 1.0 "None" false
      (:`then`
        (`AbilityAsync_WaitGameplayEvent.WaitGameplayEventToActor` (`self.Actor`) (struct :`TagName` "Montage.MagicEffect") true
          (:`EventReceived`
            (`self.SpawnProjectile` false true))))
      (:`OnCompleted`
        (`self.K2_EndAbility` :!label _label_2))
      (:`OnBlendOut`
        (goto _label_2))
      (:`OnInterrupted`
        (goto _label_2)))
    (else
      (bind _returnvalue_2 (message `CharacterInterface.GetSecondaryWeaponHandheldType` (`self.Actor`)))
      (if (`BlueprintGameplayTagLibrary.MatchesTag` _returnvalue_2 (struct :`TagName` "Handheld.Secondary.Magic.Enhance"))
        (bind _returnvalue_3 (message `CharacterInterface.GetDurability` (`self.Actor`) true))
        (if (not (== _returnvalue_3 0.0))
          (`AbilityTask_PlayMontageAndWait.CreatePlayMontageAndWaitProxy` "None" "/Game/Asset/Enemy/Warrior/Spellcast_Raise_Montage.Spellcast_Raise_Montage"
            (:`OnCompleted`
              _)
            (:`OnBlendOut`
              _)
            (:`OnInterrupted`
              _))
          (`AbilitySystemBlueprintLibrary.AddLooseGameplayTags` (`self.Actor`) (`BlueprintGameplayTagLibrary.MakeLiteralGameplayTagContainer` (struct :`GameplayTags` (struct :`(TagName` "Ability.Enhance")))))
          (message `CharacterInterface.SetDurability` (`self.Actor`) -1.0 true)
          (`self.K2_EndAbility`))
        (else
          (goto _label))))))