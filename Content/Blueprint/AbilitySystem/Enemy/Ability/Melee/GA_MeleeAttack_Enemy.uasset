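; Enemy melee attack gameplay ability that plays a randomly chosen attack montage on its avatar.
; SelectAttackMontage gets a count-to-montage map from the avatar by handheld type through an interface message, then looks up a random key from 1 to the map's length.
; The ability ends when the montage completes, blends out or is interrupted, or immediately if none is valid; ending it does not stop the montage.
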(event `self.K2_ActivateAbility`
  (bind _outmontage (`self.SelectAttackMontage`))
  (`/Engine/EditorBlueprintResources/StandardMacros.IsValid` _outmontage
    (:`Is Valid`
      (`AbilityTask_PlayMontageAndWait.CreatePlayMontageAndWaitProxy` "None" _outmontage 1.0 "None" false
        (:`OnCompleted`
          _)
        (:`OnBlendOut`
          _)
        (:`OnInterrupted`
          _))
      (`self.K2_EndAbility`))
    (:`Is Not Valid`
      (`self.K2_EndAbility`))))

(fn `SelectAttackMontage`
  (returns (OutMontage :type "AnimMontage Object Reference"))
  (locals (WeaponType :type "GameplayTag Structure") (CountToMontage :type "Map of Integer to AnimMontage Object Reference"))
  (bind _returnvalue (message `EnemyInterface.GetCountToMontageByHandheldType` (`self.GetAvatarActorFromActorInfo`)))
  (bind _output_get (set `local.CountToMontage` _returnvalue))
  (return (`BlueprintMapLibrary.Map_Find` _output_get (`KismetMathLibrary.RandomIntegerInRange` 1 (`BlueprintMapLibrary.Map_Length` _output_get)))))