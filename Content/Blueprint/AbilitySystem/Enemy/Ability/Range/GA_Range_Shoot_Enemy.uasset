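; Enemy ranged-attack gameplay ability that either fires or reloads on each activation, querying the avatar through message calls.
; If loaded, it plays the shoot montage, spawns a target-locked arrow with overridden pitch on the Montage.Shoot event, then clears the loaded state.
; Otherwise, with enough ammunition, it plays the reload montage and sets loaded, even on blend-out or interruption.
; The ability ends with the montage, or immediately without ammunition.
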(event `self.K2_ActivateAbility`
  (set `self.Actor` (`self.GetAvatarActorFromActorInfo`))
  (bind _returnvalue (message `EnemyInterface.GetIsLoaded` (`self.Actor`)))
  (if _returnvalue
    (bind _returnvalue_2 (message `EnemyInterface.GetShootMontage` (`self.Actor`) false))
    (`AbilityTask_PlayMontageAndWait.CreatePlayMontageAndWaitProxy` "None" _returnvalue_2
      (:`then`
        (`AbilityAsync_WaitGameplayEvent.WaitGameplayEventToActor` (`self.Actor`) (struct :`TagName` "Montage.Shoot") true
          (:`EventReceived`
            (`self.SpawnProjectile` false true true 15.0 true)
            (message `EnemyInterface.SetIsLoaded` (`self.Actor`) false))))
      (:`OnCompleted`
        (`self.K2_EndAbility` :!label _label))
      (:`OnBlendOut`
        (goto _label))
      (:`OnInterrupted`
        (goto _label)))
    (else
      (bind _returnvalue_3 (message `EnemyInterface.CheckAmmunitionIsEnough` (`self.Actor`)))
      (if _returnvalue_3
        (bind _returnvalue_4 (message `EnemyInterface.GetReloadMontage` (`self.Actor`)))
        (`AbilityTask_PlayMontageAndWait.CreatePlayMontageAndWaitProxy` "None" _returnvalue_4
          (:`OnCompleted`
            _)
          (:`OnBlendOut`
            _)
          (:`OnInterrupted`
            _))
        (message `EnemyInterface.SetIsLoaded` (`self.Actor`) true)
        (`self.K2_EndAbility`)
        (else
          (`self.K2_EndAbility`))))))