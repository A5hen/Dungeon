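; GA_HitReact is a shared gameplay ability that plays a hit reaction on its avatar.
; On activation it broadcasts end messages for trace checks, blocking and spinning, then applies GE_HitReact to itself.
; The triggering event's magnitude, truncated to an integer, selects the montage through an avatar message, played slightly slowed.
; When the montage completes, blends out or is interrupted, it removes the effect, clears the attacking flag and ends.
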(event `self.K2_ActivateAbility`
  (bind _returnvalue (`self.GetAbilitySystemComponentFromActorInfo`))
  (set `self.Actor` (`self.GetAvatarActorFromActorInfo`))
  (set `self.HitReactType` (`.EventMagnitude` (break `GameplayEventData` (`self.CurrentEventData`))))
  (`self.BroadcastEndDelegates`)
  (bind _returnvalue_2 (`AbilitySystemComponent.BP_ApplyGameplayEffectToSelf` _returnvalue "/Game/Blueprint/AbilitySystem/Enemy/Effect/GE_HitReact.GE_HitReact_C" 1.0 (`AbilitySystemComponent.MakeEffectContext` _returnvalue)))
  (set `self.EffectHandle` _returnvalue_2)
  (bind _returnvalue_3 (message `CharacterInterface.GetHitReactMontage` (`self.Actor`) (`KismetMathLibrary.FTrunc` (`self.HitReactType`))))
  (`AbilityTask_PlayMontageAndWait.CreatePlayMontageAndWaitProxy` "None" _returnvalue_3 0.8
    (:`OnCompleted`
      _)
    (:`OnBlendOut`
      _)
    (:`OnInterrupted`
      _))
  (`AbilitySystemComponent.RemoveActiveGameplayEffect` (`self.GetAbilitySystemComponentFromActorInfo`) (`self.EffectHandle`) -1)
  (message `PlayerInterface.SetIsAttacking` (`self.Actor`) false)
  (`self.K2_EndAbility`))

(fn `BroadcastEndDelegates`
  (message `CharacterInterface.BroadcastTraceCheckEndDelegate` (`self.GetAvatarActorFromActorInfo`))
  (message `CharacterInterface.BroadcastBlockingEndDelegate` (`self.GetAvatarActorFromActorInfo`))
  (message `CharacterInterface.BroadcastSpinningEndDelegate` (`self.GetAvatarActorFromActorInfo`)))