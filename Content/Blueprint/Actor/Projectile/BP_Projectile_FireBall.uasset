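; Fireball projectile Blueprint that stops homing on its target shortly after a homing-end notification.
; On BeginPlay it binds a handler to the OnHomingEnd event dispatcher.
; After a short delay, the handler disables homing on ProjectileMovement and resets velocity to a fixed speed along the current direction, so the fireball continues without steering.
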(event `self.ReceiveBeginPlay`
  (add `self.OnHomingEnd` (delegate `OnHomingEnd_事件`)))

(event `OnHomingEnd_事件`
  (`KismetSystemLibrary.Delay` 0.6)
  (set `ProjectileMovementComponent.bIsHomingProjectile` false (`self.ProjectileMovement`))
  (set `MovementComponent.Velocity` (* (`KismetMathLibrary.Normal` (`MovementComponent.Velocity` (`self.ProjectileMovement`))) 200) (`self.ProjectileMovement`)))

(fn `UserConstructionScript`)