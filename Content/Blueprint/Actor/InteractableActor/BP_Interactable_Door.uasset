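; Interactable door actor that swings open or closed when its interaction event starts, showing an "E" key prompt on its icon.
; Each interaction stores the current actor yaw, flips InteractBool and plays the Door timeline from the start.
; The timeline's Angle is added to or subtracted from that yaw, depending on InteractBool, to rotate the mesh.
; InitializeStatus snaps the mesh to the actor's yaw, offset 90 degrees when InteractBool is true.
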(event `SaveInterface.InitializeStatus`
  (`self.InitializeByBool` (`self.InteractBool`)))

(event `self.ReceiveBeginPlay`
  (message `/Game/Blueprint/Interaction/BPI_UIAux.SetKeyName` (`WidgetComponent.GetUserWidgetObject` (`self.InteractIcon`)) "E")
  (add `self.OnEventStart` (delegate `OnEventStart_事件`)))

(event `OnEventStart_事件`
  (bind (_returnvalue_roll _returnvalue_pitch) (`KismetMathLibrary.BreakRotator` (`self.K2_GetActorRotation` self)))
  (bind (_returnvalue_roll_2 _returnvalue_pitch_2 _returnvalue_yaw) (`KismetMathLibrary.BreakRotator` (`self.K2_GetActorRotation` self)))
  (set `self.CurrentZ` _returnvalue_yaw)
  (if (`self.InteractBool`)
    (set `self.InteractBool` false)
    (bind (_direction _angle) (`Timeline|Door` :!via `PlayFromStart` :!label _label)
      (:`Update`
        (bind _outfloat (`self.UpdateByBool` _angle (`self.InteractBool`)))
        (`SceneComponent.K2_SetWorldRotation` (`self.StaticMeshComponent`) (`KismetMathLibrary.MakeRotator` _returnvalue_roll _returnvalue_pitch _outfloat) false false)))
    (else
      (set `self.InteractBool` true)
      (goto _label :!via `PlayFromStart`))))

(fn `InitializeByBool`
  (params (InBool :type Boolean))
  (locals (Out :type "Float (double-precision)"))
  (bind (_returnvalue_roll _returnvalue_pitch _returnvalue_yaw) (`KismetMathLibrary.BreakRotator` (`self.K2_GetActorRotation` self)))
  (if InBool
    (bind _output_get (set `local.Out` (+ _returnvalue_yaw 90.0)))
    (`SceneComponent.K2_SetWorldRotation` (`self.StaticMeshComponent`) (`KismetMathLibrary.MakeRotator` _returnvalue_roll _returnvalue_pitch _output_get) false false)
    (else
      (`SceneComponent.K2_SetWorldRotation` (`self.StaticMeshComponent`) (`KismetMathLibrary.MakeRotator` _returnvalue_roll _returnvalue_pitch _returnvalue_yaw) false false))))

(fn `UpdateByBool`
  (params (InFloat :type "Float (double-precision)") (InBool :type Boolean))
  (returns (OutFloat :type "Float (double-precision)"))
  (locals (UpdateFloat :type "Float (double-precision)"))
  (set `local.UpdateFloat` InFloat)
  (if InBool
    (return (+ (`self.CurrentZ`) (`local.UpdateFloat`)))
    (else
      (return (- (`self.CurrentZ`) (`local.UpdateFloat`))))))

(fn `UserConstructionScript`)