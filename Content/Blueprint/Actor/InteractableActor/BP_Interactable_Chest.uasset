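; Interactable chest actor whose lid swings open once when the player triggers its interaction event.
; On BeginPlay it sets an "E" key prompt and, if not yet used, binds OnEventStart, which sets InteractBool and plays a timeline rolling BoxUpper open.
; The timeline update unbinds the event and hides the prompt.
; InitializeStatus snaps used chests open, and the construction script previews the lid from the Open flag.
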(event `SaveInterface.InitializeStatus`
  (bind (_returnvalue_roll _returnvalue_pitch _returnvalue_yaw) (`KismetMathLibrary.BreakRotator` (`self.K2_GetActorRotation`)))
  (if (`self.InteractBool`)
    (`SceneComponent.K2_SetWorldRotation` (`self.Box_Upper`) (`KismetMathLibrary.MakeRotator` (- _returnvalue_roll 60.0) _returnvalue_pitch _returnvalue_yaw) false false)))

(event `self.ReceiveBeginPlay`
  (message `/Game/Blueprint/Interaction/BPI_UIAux.SetKeyName` (`WidgetComponent.GetUserWidgetObject` (`self.InteractIcon`)) "E")
  (if (not (`self.InteractBool`))
    (add `self.OnEventStart` (delegate `OnEventStart_事件`))))

(event `OnEventStart_事件`
  (bind (_returnvalue_roll _returnvalue_pitch _returnvalue_yaw) (`KismetMathLibrary.BreakRotator` (`self.K2_GetActorRotation`)))
  (set `self.InteractBool` true)
  (bind (_direction _angle) (`Timeline|Chest` :!via `PlayFromStart`)
    (:`Update`
      (`SceneComponent.K2_SetWorldRotation` (`self.Box_Upper`) (`KismetMathLibrary.MakeRotator` (- _returnvalue_roll _angle) _returnvalue_pitch _returnvalue_yaw) false false)
      (clear `self.OnEventStart`)
      (set `Widget.RenderOpacity` 0.0 (`WidgetComponent.GetUserWidgetObject` (`self.InteractIcon`))))))

(fn `UserConstructionScript`
  (bind (_returnvalue_roll _returnvalue_pitch _returnvalue_yaw) (`KismetMathLibrary.BreakRotator` (`self.K2_GetActorRotation`)))
  (bind (_returnvalue_roll_2 _returnvalue_pitch_2 _returnvalue_yaw_2) (`KismetMathLibrary.BreakRotator` (`self.K2_GetActorRotation`)))
  (if (`self.Open`)
    (`SceneComponent.K2_SetWorldRotation` (`self.Box_Upper`) (`KismetMathLibrary.MakeRotator` (- _returnvalue_roll 60.0) _returnvalue_pitch _returnvalue_yaw) false false)
    (else
      (`SceneComponent.K2_SetWorldRotation` (`self.Box_Upper`) (`KismetMathLibrary.MakeRotator` _returnvalue_roll_2 _returnvalue_pitch_2 _returnvalue_yaw_2) false false))))