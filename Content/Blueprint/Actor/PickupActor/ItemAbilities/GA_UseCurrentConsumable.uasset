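; Gameplay ability that uses the avatar's current consumable item.
; It queries the avatar through messages, proceeding only when IsCurrentConsumableEmpty returns true and GetIsTargetToItem returns false; otherwise it ends immediately.
; It then sends UseCurrentConsumable and plays the use-item montage, which is not stopped by ability end.
; The ability ends when the montage completes, blends out or is interrupted.
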(event `self.K2_ActivateAbility`
  (bind _returnvalue (message `PlayerInterface.IsCurrentConsumableEmpty` (`self.GetAvatarActorFromActorInfo`)))
  (if _returnvalue
    (bind _returnvalue_2 (message `PlayerInterface.GetIsTargetToItem` (`self.GetAvatarActorFromActorInfo`)))
    (if _returnvalue_2
      (`self.K2_EndAbility`)
      (else
        (message `PlayerInterface.UseCurrentConsumable` (`self.GetAvatarActorFromActorInfo`))
        (`AbilityTask_PlayMontageAndWait.CreatePlayMontageAndWaitProxy` "None" "/Game/Asset/Character/Knight/Use_Item_Montage.Use_Item_Montage" 1.0 "None" false
          (:`OnCompleted`
            _)
          (:`OnBlendOut`
            _)
          (:`OnInterrupted`
            _))
        (`self.K2_EndAbility`)))
    (else
      (`self.K2_EndAbility`))))