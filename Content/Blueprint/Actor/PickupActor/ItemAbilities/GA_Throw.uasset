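; Gameplay ability for aiming and throwing the avatar's current consumable item.
; After consumable and item-target checks, it releases lock-on, then shows an aim spline with controller-driven yaw while input is held.
; Specific-input tasks cancel or switch throw angle; release plays a montage.
; The Montage.Throw event or montage interruption commits cost, spawns the projectile and uses the item; EndThrow restores state and commits cooldown.
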(event `self.K2_ActivateAbility`
  (bind _returnvalue (`self.GetAvatarActorFromActorInfo`))
  (bind _returnvalue_2 (message `PlayerInterface.IsCurrentConsumableEmpty` (`self.GetAvatarActorFromActorInfo`)))
  (if _returnvalue_2
    (bind _returnvalue_3 (message `PlayerInterface.GetIsTargetToItem` (`self.GetAvatarActorFromActorInfo`)))
    (if _returnvalue_3
      (`self.K2_EndAbility`)
      (else
        (`self.EndLock`)
        (`AbilityTask_WaitInputRelease.WaitInputRelease` false
          (:`then`
            (message `PlayerInterface.SetShowAuxSpline` (`self.GetAvatarActorFromActorInfo`) true)
            (message `PlayerInterface.SetUseControllerRotationYaw` (`self.GetAvatarActorFromActorInfo`) true)
            (bind _asynctaskproxy (`SpecificInputTask.CreateUSpecificInputTask` (`self.EndTag`))
              (:`then`
                (set `self.EndTask` _asynctaskproxy)
                (bind _asynctaskproxy_2 (`SpecificInputTask.CreateUSpecificInputTask` (`self.SwitchTag`))
                  (:`then`
                    (set `self.SwitchTask` _asynctaskproxy_2))
                  (:`OnSpecificInput`
                    (message `PlayerInterface.SwitchThrowAngle` (`self.GetAvatarActorFromActorInfo`)))))
              (:`OnSpecificInput`
                (`self.EndThrow`))))
          (:`OnRelease`
            (`AbilityTask_PlayMontageAndWait.CreatePlayMontageAndWaitProxy` "None" "/Game/Asset/Character/Knight/Throw_Montage.Throw_Montage" 1.0 "None" false
              (:`then`
                (message `PlayerInterface.SetShowAuxSpline` _returnvalue false)
                (message `PlayerInterface.EndShowAuxSpline` _returnvalue)
                (`AbilityAsync_WaitGameplayEvent.WaitGameplayEventToActor` (`self.GetAvatarActorFromActorInfo`) (struct :`TagName` "Montage.Throw") true
                  (:`EventReceived`
                    (`self.K2_CommitAbilityCost` false :!label _label)
                    (`self.SpawnActor_Throw`)
                    (message `PlayerInterface.UseCurrentConsumable` (`self.GetAvatarActorFromActorInfo`))
                    (`self.EndThrow`))))
              (:`OnCompleted`
                (`self.EndThrow` :!label _label_2))
              (:`OnBlendOut`
                (goto _label_2))
              (:`OnInterrupted`
                (goto _label)))))))
    (else
      (`self.K2_EndAbility`))))

(fn `EndLock`
  (message `PlayerInterface.SetIsLocking` (`self.GetAvatarActorFromActorInfo`) false)
  (bind _returnvalue (message `PlayerInterface.GetCharacterMovementComponent` (`self.GetAvatarActorFromActorInfo`)))
  (set `CharacterMovementComponent.bUseControllerDesiredRotation` false _returnvalue)
  (set `CharacterMovementComponent.bOrientRotationToMovement` true _returnvalue)
  (message `PlayerInterface.SetSpringArmOffset` (`self.GetAvatarActorFromActorInfo`) 0.0 0.0 35.0))

(fn `EndThrow`
  (bind _returnvalue (`self.GetAvatarActorFromActorInfo`))
  (message `PlayerInterface.SetShowAuxSpline` _returnvalue false)
  (message `PlayerInterface.EndShowAuxSpline` _returnvalue)
  (message `PlayerInterface.SetUseControllerRotationYaw` (`self.GetAvatarActorFromActorInfo`) false)
  (bind _endtask (`self.EndTask`)
    (:`then`
      (`GameplayTask.EndTask` _endtask))
    (:`else`
      _))
  (bind _switchtask (`self.SwitchTask`)
    (:`then`
      (`GameplayTask.EndTask` _switchtask))
    (:`else`
      _))
  (`self.K2_CommitAbilityCooldown` false)
  (`self.K2_EndAbility`))