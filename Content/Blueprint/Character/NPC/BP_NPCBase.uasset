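; Base NPC Blueprint that shows an "E" interact key icon and opens or closes a shop when its start event fires.
; Opening creates WBP_Shop with a shop widget controller, positions it relative to the viewport and enables the cursor with game-and-UI input.
; Closing removes the widget and restores game-only input unless the in-range player's Menu is open, using per-widget open flags on that player.
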(event `self.ReceiveBeginPlay`
  (message `/Game/Blueprint/Interaction/BPI_UIAux.SetKeyName` (`WidgetComponent.GetUserWidgetObject` (`self.InteractIcon`)) "E")
  (add `self.OnEventStart` (delegate `OnEventStart_事件`))
  (add `self.CloseShop` (delegate `CloseShop_事件`)))

(event `OnEventStart_事件`
  (bind _returnvalue (`GameplayStatics.GetPlayerController` 0))
  (bind _shopwidget (`self.ShopWidget`))
  (bind (_x _y) (`KismetMathLibrary.BreakVector2D` (`WidgetLayoutLibrary.GetViewportSize`)))
  (if (`self.IsShopOpen`)
    (`self.CloseShop_事件`)
    (else
      (bind _returnvalue_2 (`|CreateWidget` "/Game/Blueprint/UI/Shop/WBP_Shop.WBP_Shop_C"))
      (set `self.ShopWidget` _returnvalue_2)
      (`PlayerUserWidget.SetWidgetController` (`self.ShopWidget`) (`DungeonAbilitySystemLibrary.GetShopWidgetController` null self))
      (`UserWidget.AddToViewport` _shopwidget 1)
      (`UserWidget.SetDesiredSizeInViewport` _shopwidget (600.0 300.0))
      (`UserWidget.SetPositionInViewport` (`self.ShopWidget`) (`KismetMathLibrary.MakeVector2D` (* _x 0.35) (* _y 0.1)) true)
      (set `self.IsShopOpen` true)
      (bind _returnvalue_3 (`self.GetPlayerInRange`))
      (message `PlayerInterface.SetWidgetOpen` _returnvalue_3 true "Shop")
      (set `PlayerController.bShowMouseCursor` true _returnvalue)
      (`WidgetBlueprintLibrary.SetInputMode_GameAndUIEx` _returnvalue null "DoNotLock" false))))

(event `CloseShop_事件`
  (bind _returnvalue (`GameplayStatics.GetPlayerController` 0))
  (bind _shopwidget (`self.ShopWidget`)
    (:`then`
      (`Widget.RemoveFromParent` _shopwidget))
    (:`else`
      _))
  (set `self.IsShopOpen` false)
  (bind _returnvalue_2 (`self.GetPlayerInRange`))
  (message `PlayerInterface.SetWidgetOpen` _returnvalue_2 false "Shop")
  (bind _returnvalue_3 (`self.GetPlayerInRange`))
  (bind _returnvalue_4 (message `PlayerInterface.GetIsWidgetOpen` _returnvalue_3 "Menu"))
  (if (not _returnvalue_4)
    (set `PlayerController.bShowMouseCursor` false _returnvalue)
    (`WidgetBlueprintLibrary.SetInputMode_GameOnly` _returnvalue)))

(fn `UserConstructionScript`)