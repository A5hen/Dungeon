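; Warrior enemy Blueprint that turns to face its target player while awake.
; Each tick, if IsAwake is set, it stores the result of GetTargetActor in TargetPlayer and, when valid, smoothly interpolates its rotation toward that actor using only the look-at yaw.
; BeginPlay and construction only call the parent, and the overlap event is disabled.
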(event `self.ReceiveBeginPlay`
  (`parent.ReceiveBeginPlay`))

(event `self.ReceiveTick`
  (params (DeltaSeconds :type "Float (single-precision)"))
  (bind (_returnvalue_roll _returnvalue_pitch _returnvalue_yaw) (`KismetMathLibrary.BreakRotator` (`KismetMathLibrary.FindLookAtRotation` (`self.K2_GetActorLocation`) (`self.K2_GetActorLocation` (`self.TargetPlayer`)))))
  (if (`self.IsAwake`)
    (bind _returnvalue (`CharacterInterface.GetTargetActor` self))
    (bind _output_get (set `self.TargetPlayer` _returnvalue))
    (`/Engine/EditorBlueprintResources/StandardMacros.IsValid` _output_get
      (:`Is Valid`
        (`self.K2_SetActorRotation` (`KismetMathLibrary.RInterpTo` (`self.K2_GetActorRotation`) (`KismetMathLibrary.MakeRotator` 0.0 0.0 _returnvalue_yaw) (`GameplayStatics.GetWorldDeltaSeconds`) 5.0))))))

(fn `UserConstructionScript`
  (`parent.UserConstructionScript`))