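; BP_Kight is the player knight Blueprint, layering death UI, lock-on camera and throw aiming onto its parent class.
; Death shows WBP_Death with UI-only input, then calls HandleDie after a delay.
; Tick runs falling checks, turns control rotation toward the locked target and, while aiming, rebuilds spline meshes along the predicted throw arc each frame.
; Events also toggle throw angle, move the camera boom and set physics rotation during root motion.
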(event `self.Die_BlueprintImplement`
  (bind _returnvalue (`|CreateWidget` "/Game/Blueprint/UI/WBP_Death.WBP_Death_C"))
  (`UserWidget.AddToViewport` _returnvalue 10)
  (`WidgetBlueprintLibrary.SetInputMode_UIOnlyEx` (`GameplayStatics.GetPlayerController` 0) _returnvalue)
  (`KismetSystemLibrary.Delay` 3.0)
  (`self.HandleDie`))

(event `PlayerInterface.AllowRootMotion`
  (params (InBool :type Boolean))
  (set `CharacterMovementComponent.bAllowPhysicsRotationDuringAnimRootMotion` InBool (`self.CharacterMovement`)))

(event `PlayerInterface.SetSpringArmOffset`
  (params (X :type "Float (single-precision)") (Y :type "Float (single-precision)") (Z :type "Float (single-precision)"))
  (`SceneComponent.K2_SetRelativeLocation` (`self.CameraBoom`) (`KismetMathLibrary.MakeVector` X Y Z) false false))

(event `self.ReceiveTick`
  (params (DeltaSeconds :type "Float (single-precision)"))
  (bind _spline (`self.Spline`))
  (bind _splinepoints (`self.SplinePoints`))
  (`self.TickForFalling`)
  (`self.TickForLockTarget`)
  (if (`self.bShowAuxSpline`)
    (for _array_element _splinepoints
      (`ActorComponent.K2_DestroyComponent` _array_element))
    (`KismetArrayLibrary.Array_Clear` _splinepoints)
    (bind _returnvalue (`PlayerInterface.GetThrowVelocity` self))
    (bind _returnvalue_2 (`self.TickForThrow` (`SceneComponent.K2_GetComponentLocation` (`self.ThrowPoint`)) _returnvalue))
    (for _index (range (+ _returnvalue_2 1))
      (bind _returnvalue_3 (`AddComponent|NODE_AddSplineMeshComponent-0` :`bManualAttachment` true))
      (`SplineMeshComponent.SetStartScale` _returnvalue_3 (0.01 0.01) true)
      (`SplineMeshComponent.SetEndScale` _returnvalue_3 (0.01 0.01) true)
      (bind (_location _tangent) (`SplineComponent.GetLocationAndTangentAtSplinePoint` _spline _index "Local"))
      (bind (_location_2 _tangent_2) (`SplineComponent.GetLocationAndTangentAtSplinePoint` _spline (+ _index 1) "Local"))
      (`SplineMeshComponent.SetStartAndEnd` _returnvalue_3 _location _tangent _location_2 _tangent_2 true)
      (`KismetArrayLibrary.Array_Add` (`self.SplinePoints`) _returnvalue_3))))

(event `PlayerInterface.EndShowAuxSpline`
  (bind _splinepoints (`self.SplinePoints`))
  (for _array_element _splinepoints
    (`ActorComponent.K2_DestroyComponent` _array_element))
  (`KismetArrayLibrary.Array_Clear` _splinepoints))

(event `PlayerInterface.SwitchThrowAngle`
  (if (`self.IsLowerAngle`)
    (`SceneComponent.K2_SetRelativeRotation` (`self.ThrowPoint`) (struct :`Pitch` 60.0 :`Yaw` 90.0) false false)
    (set `self.IsLowerAngle` false)
    (else
      (`SceneComponent.K2_SetRelativeRotation` (`self.ThrowPoint`) (struct :`Pitch` 25.0 :`Yaw` 90.0) false false)
      (set `self.IsLowerAngle` true))))

(fn `TickForLockTarget`
  (if (`self.IsLocking`)
    (`/Engine/EditorBlueprintResources/StandardMacros.IsValid` (`self.LockTarget`)
      (:`Is Valid`
        (`Controller.SetControlRotation` (`GameplayStatics.GetPlayerController` 0) (`KismetMathLibrary.RInterpTo` (`self.GetControlRotation`) (`KismetMathLibrary.MakeRotator` 0.0 -20.0 (.yaw (`KismetMathLibrary.FindLookAtRotation` (`PlayerCameraManager.GetCameraLocation` (`PlayerController.PlayerCameraManager` (`GameplayStatics.GetPlayerController` 0))) (`self.K2_GetActorLocation` (`self.LockTarget`))))) (`GameplayStatics.GetWorldDeltaSeconds`) 10.0))))))

(fn `UserConstructionScript`
  (`parent.UserConstructionScript`))